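; Zombie enemy that patrols by walking forward every Tick and turning around when its WallDetection trigger overlaps, with a short cooldown between turns.
; The DetectDaño trigger deals fixed damage to BP_Eira on overlap.
; AnyDamage lowers VidaZombie and destroys the actor at zero.
; BeginPlay caches the UW_EnemyHealth widget, but UpdateHealthBar is empty; AIMoveTo logic also exists, though StartMovement is not called here.
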(event `ZombieMuerto`
  (`self.K2_DestroyActor`))

(event `self.ReceiveAnyDamage`
  (params (Damage :type "Float (single-precision)") (DamageType :type "DamageType Object Reference") (InstigatedBy :type "Controller Object Reference") (DamageCauser :type "Actor Object Reference"))
  (bind _output_get (set `self.VidaZombie` (- (`self.VidaZombie`) Damage)))
  (if (<= _output_get 0.0)
    (`self.ZombieMuerto`)))

(event `UpdateHealthBar`)

(event `StartMovement`
  (bind _asaic_zombie (cast `/Game/Blueprints/AIC_Zombie` (`self.GetController`)))
  (`|AIMoveTo` _asaic_zombie self (+ (`self.K2_GetActorLocation`) (`KismetMathLibrary.MakeVector` 1000.0)) null
    (:`OnSuccess`
      (`self.StartMovement`))))

(event `self.ReceiveBeginPlay`
  (`|ExecutionSequence`
    (:`then_0`
      (bind _asuw_enemy_health (cast `/Game/Textures/OBJS/Enemies/UW_EnemyHealth` (`WidgetComponent.GetUserWidgetObject` (`self.Widget`)))
        (:`then`
          (set `self.HealthBarRef` _asuw_enemy_health))
        (:`CastFailed`
          (`KismetSystemLibrary.PrintString` "error"))))
    (:`then_1`
      (`|AIMoveTo` self (1.0 0.0 0.0) (`self.GetController`)))))

(event `self.ReceiveTick`
  (params (DeltaSeconds :type "Float (single-precision)"))
  (`self.AddMovementInput` (`self.GetActorForwardVector`)))

(event `self.WallDetection.OnComponentBeginOverlap`
  (params (OverlappedComponent :type "PrimitiveComponent Object Reference") (OtherActor :type "Actor Object Reference") (OtherComp :type "PrimitiveComponent Object Reference") (OtherBodyIndex :type Integer) (bFromSweep :type Boolean) (SweepResult :type "HitResult Structure (by ref)"))
  (if (`self.Rotation`)
    (`self.TurnChar`)))

(event `self.DetectDaño.OnComponentBeginOverlap`
  (params (OverlappedComponent :type "PrimitiveComponent Object Reference") (OtherActor :type "Actor Object Reference") (OtherComp :type "PrimitiveComponent Object Reference") (OtherBodyIndex :type Integer) (bFromSweep :type Boolean) (SweepResult :type "HitResult Structure (by ref)"))
  (bind _asbp_eira (cast `/Game/Blueprints/BP_Eira` OtherActor))
  (`GameplayStatics.ApplyDamage` _asbp_eira 20.0 null self))

(event `TurnChar`
  (`self.K2_SetActorRotation` (`KismetMathLibrary.ComposeRotators` (`self.K2_GetActorRotation` self) (struct :`Yaw` 180.0)))
  (set `self.Rotation` false)
  (`KismetSystemLibrary.Delay` 0.2)
  (set `self.Rotation` true))

(fn `DañoRecibido`
  (params (`DañoCant` :type "Float (double-precision)"))
  (set `self.VidaZombie` (- (`self.VidaZombie`) `DañoCant`)))

(fn `EsconderBarra`
  (`SceneComponent.SetVisibility` (`self.Widget`) false false))

(fn `UserConstructionScript`)