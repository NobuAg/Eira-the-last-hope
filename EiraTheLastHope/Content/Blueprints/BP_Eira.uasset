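; BP_Eira is the player character for a side-scrolling game, with lateral movement, jump, crouch and bow attacks that spawn BP_Arrow.
; Damage lowers Vida and triggers knockback plus timed invulnerability, or death and a Game Over widget.
; It creates the HUD, pause, checkpoint and level-finish widgets, and saves or restores its transform through BP_SaveGame.
; State flags track attack, crouch, hurt, death, movement and long idle.
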(event `SaveGame`
  (bind _bp_savegame (`self.BP_SaveGame`))
  (bind _returnvalue (`GameplayStatics.DoesSaveGameExist` "Save1"))
  (if _returnvalue
    (set `/Game/Blueprints/BP_SaveGame.ActorTransform` (`self.GetTransform`) _bp_savegame)
    (`GameplayStatics.SaveGameToSlot` _bp_savegame "Save1")))

(event `IniSaveGame`
  (bind _returnvalue (`GameplayStatics.DoesSaveGameExist` "Save1"))
  (if _returnvalue
    (bind _returnvalue_2 (`GameplayStatics.LoadGameFromSlot` "Save1"))
    (bind _asbp_save_game (cast `/Game/Blueprints/BP_SaveGame` _returnvalue_2))
    (bind _output_get (set `self.BP_SaveGame` _asbp_save_game))
    (`self.K2_SetActorTransform` (`/Game/Blueprints/BP_SaveGame.ActorTransform` _output_get))
    (`KismetSystemLibrary.PrintString` "LoadGame")
    (else
      (bind _returnvalue_3 (`GameplayStatics.CreateSaveGameObject` "/Game/Blueprints/BP_SaveGame.BP_SaveGame_C"))
      (bind _output_get_2 (set `self.BP_SaveGame` _returnvalue_3))
      (`GameplayStatics.SaveGameToSlot` _output_get_2 "Save1")
      (set `/Game/Blueprints/BP_SaveGame.ActorTransform` (`self.GetTransform`) (`self.BP_SaveGame`))
      (`KismetSystemLibrary.PrintString` "NewSave"))))

(event `InputAction|Pause` :paused true
  (params (Key :type "Key Structure"))
  ; Pause
  (:`Pressed`
    (if (not (`self.IsPaused?`))
      (bind _returnvalue (`|GenericCreateObject` "/Game/Blueprints/Menu/UW_Pause.UW_Pause_C" null))
      (set `self.UWPause` _returnvalue)
      (`UserWidget.AddToViewport` _returnvalue 0)
      (`GameplayStatics.SetGamePaused` true)
      (`WidgetBlueprintLibrary.SetInputMode_GameAndUIEx` (`GameplayStatics.GetPlayerController` 0) _returnvalue))))

(event `InputAction|AtaqueArco`
  (params (Key :type "Key Structure"))
  ; Spawn a la flecha del ataque
  (:`Pressed`
    (set `self.IsAttacking` true)
    (`|SpawnActorFromClass` "/Game/Textures/Characters/Eira/Animations/BP_Arrow.BP_Arrow_C" (`SceneComponent.K2_GetComponentToWorld` (`self.ArrowSpawn`)) "AlwaysSpawn" "MultiplyWithRoot" self null))
  (:`Released`
    (set `self.IsAttacking` false)
    (set `self.ShouldReturnToIdle` true)))

(event `TextBoxBoss`)

(event `MuerteChar`
  (`self.DisableInput` (`GameplayStatics.GetPlayerController` 0))
  (set `self.Death` true)
  (bind _returnvalue (`|CreateWidget` "/Game/Blueprints/UW_GameOver.UW_GameOver_C"))
  (`UserWidget.AddToViewport` _returnvalue 0)
  (`WidgetBlueprintLibrary.SetInputMode_GameAndUIEx` (`GameplayStatics.GetPlayerController` 0) _returnvalue))

(event `self.ReceiveAnyDamage`
  (params (Damage :type "Float (single-precision)") (DamageType :type "DamageType Object Reference") (InstigatedBy :type "Controller Object Reference") (DamageCauser :type "Actor Object Reference"))
  ; Logica de daño recibido e invunerabilidad
  (`/Engine/EditorBlueprintResources/StandardMacros.IsValid` DamageCauser
    (:`Is Valid`
      (if (not (`self.Invencible`))
        (set `self.IsHurt` true)
        (bind _output_get (set `self.Vida` (- (`self.Vida`) Damage)))
        (`|ExecutionSequence`
          (:`then_0`
            (if (<= _output_get 0.0)
              (`self.MuerteChar`)
              (else
                (set `self.Death` false))))
          (:`then_1`
            (`KismetSystemLibrary.Delay` 0.2)
            (`self.LaunchCharacter` (* (200.0 0.0 0.0) (.x (`KismetMathLibrary.Vector_Normal2D` (- (`self.K2_GetActorLocation` self) (`self.K2_GetActorLocation` DamageCauser))))))
            (set `self.IsHurt` false)
            (set `self.Invencible` true)
            (`KismetSystemLibrary.K2_SetTimerDelegate` (delegate `End`) 3.0)))))
    (:`Is Not Valid`
      (`self.LaunchCharacter` (* (-200.0 0.0 0.0) (.x (`KismetMathLibrary.Normal` (* (`self.GetActorForwardVector`) -1.0))))))))

(event `End`
  ; Logica de daño recibido e invunerabilidad
  (set `self.Invencible` false))

(event `FinLevel`
  (if (`self.Nivel1??`)
    (bind _returnvalue (`|CreateWidget` "/Game/Blueprints/UW_LevelFinish.UW_LevelFinish_C"))
    (`UserWidget.AddToViewport` _returnvalue 0)
    (else
      (`self.FinLevel2`))))

(event `FinLevel2`
  (bind _returnvalue (`|CreateWidget` "/Game/Blueprints/UW_LevelFinish2.UW_LevelFinish2_C"))
  (`UserWidget.AddToViewport` _returnvalue 0))

(event `InputAxis|DesplazamientoLateral`
  (params (AxisValue :type "Float (single-precision)"))
  ; Movimiento X Y
  (`self.AddMovementInput` (1.0 0.0 0.0) AxisValue)
  (`self.Turn`)
  (set `self.Semueve?` (!= AxisValue 0.0))
  (set `self.IsIdleLong` false))

(event `FinGame`
  (bind _returnvalue (`|CreateWidget` "/Game/Blueprints/UW_FinishGame.UW_FinishGame_C"))
  (`UserWidget.AddToViewport` _returnvalue 0))

(event `FinInvensible`
  (set `self.IsHurt` false)
  (set `self.Invencible` false))

(event `self.ReceiveBeginPlay`
  (bind _returnvalue (`|CreateWidget` "/Game/Blueprints/UW_HUD.UW_HUD_C"))
  (`UserWidget.AddToViewport` _returnvalue 0))

(event `InputAction|Salto`
  (params (Key :type "Key Structure"))
  ; Salto
  (:`Pressed`
    (`self.Jump`))
  (:`Released`
    (`self.StopJumping`)))

(event `InputAction|Agacharse`
  (params (Key :type "Key Structure"))
  ; Agacharse
  (:`Pressed`
    (set `self.IsCrounching` true)
    (`self.Crouch`))
  (:`Released`
    (set `self.IsCrounching` false)
    (`self.UnCrouch`)))

(event `self.ReceiveTick`
  (params (DeltaSeconds :type "Float (single-precision)"))
  (`KismetSystemLibrary.Delay` 5.0)
  (`/Engine/EditorBlueprintResources/StandardMacros.DoOnce` false
    (:`Completed`
      (if (`self.Semueve?`)
        (`KismetSystemLibrary.K2_ClearAndInvalidateTimerHandle` (`self.IdleTimerHandle`))
        (set `self.IsIdleLong` false)
        (else
          (bind _returnvalue (`KismetSystemLibrary.K2_SetTimerDelegate` (delegate `StartLongIdleAnimation`) 5.0))
          (set `self.IdleTimerHandle` _returnvalue)
          (set `self.IsIdleLong` true))))))

(event `StartLongIdleAnimation`)

(event `self.CapsuleComponent.OnComponentBeginOverlap`
  (params (OverlappedComponent :type "PrimitiveComponent Object Reference") (OtherActor :type "Actor Object Reference") (OtherComp :type "PrimitiveComponent Object Reference") (OtherBodyIndex :type Integer) (bFromSweep :type Boolean) (SweepResult :type "HitResult Structure (by ref)"))
  (cast `/Game/Blueprints/BP_Checkpoint` OtherActor)
  (set `self.CheckpointDetect` true))

(event `InputAction|Checkpoint`
  (params (Key :type "Key Structure"))
  (:`Pressed`
    (if (`self.CheckpointDetect`)
      (bind _returnvalue (`|CreateWidget` "/Game/Blueprints/UW_MenuCheckpoint.UW_MenuCheckpoint_C"))
      (bind _output_get (set `self.WIdCheckRef` _returnvalue))
      (`UserWidget.AddToViewport` _output_get 0)
      (`WidgetBlueprintLibrary.SetInputMode_GameAndUIEx` (`GameplayStatics.GetPlayerController` 0) (`self.WIdCheckRef`)))))

(fn `Daño`
  (params (`CantidadDaño` :type "Float (double-precision)" :default 10.0) (Empuje :type "Vector Structure"))
  (set `self.Vida` (- (`self.Vida`) `CantidadDaño`)))

(fn `FinInvencible`
  (set `self.IsHurt` false))

(fn `Muerte`)

(fn `ReturnToIdle1Function`)

(fn `Turn`
  (bind _returnvalue (`self.GetController`))
  (`/Engine/EditorBlueprintResources/StandardMacros.IsValid` _returnvalue
    (:`Is Valid`
      (`/Engine/EditorBlueprintResources/StandardMacros.CompareFloat` (`self.GetInputAxisValue`)
        (:`>`
          (`Controller.SetControlRotation` _returnvalue (`KismetMathLibrary.MakeRotator` 0.0)))
        (:`<`
          (`Controller.SetControlRotation` _returnvalue (`KismetMathLibrary.MakeRotator` 0.0 0.0 -180.0)))))))

(fn `UserConstructionScript`)