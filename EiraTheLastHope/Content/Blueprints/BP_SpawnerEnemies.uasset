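; Enemy spawner actor that periodically spawns BP_Zombie enemies at random points within its Box component.
; BeginPlay spawns one zombie immediately, ignoring collisions, and starts a looping timer that calls SpawnZombie every few seconds.
; Each spawn picks a random XY offset within the box's scaled extent at the box's center height.
; Timed spawns nudge clear of collisions or skip spawning when blocked.
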(event `self.ReceiveBeginPlay`
  (bind (_returnvalue_x _returnvalue_y) (`KismetMathLibrary.BreakVector` (`BoxComponent.GetScaledBoxExtent` (`self.Box`))))
  (`KismetSystemLibrary.K2_SetTimer` null "SpawnZombie" 3.0 true)
  (`|SpawnActorFromClass` "/Game/Textures/OBJS/Enemies/BP_Zombie.BP_Zombie_C" (`KismetMathLibrary.MakeTransform` (+ (`KismetMathLibrary.MakeVector` (`KismetMathLibrary.RandomFloatInRange` (* _returnvalue_x -1.0) _returnvalue_x) (`KismetMathLibrary.RandomFloatInRange` (* _returnvalue_y -1.0) _returnvalue_y)) (`SceneComponent.K2_GetComponentLocation` (`self.Box`)))) "AlwaysSpawn" "MultiplyWithRoot" null 10.0 10.0 null))

(fn `SpawnZombie`
  (bind (_returnvalue_x _returnvalue_y) (`KismetMathLibrary.BreakVector` (`BoxComponent.GetScaledBoxExtent` (`self.Box`))))
  (`|SpawnActorFromClass` "/Game/Textures/OBJS/Enemies/BP_Zombie.BP_Zombie_C" (`KismetMathLibrary.MakeTransform` (+ (`KismetMathLibrary.MakeVector` (`KismetMathLibrary.RandomFloatInRange` (* _returnvalue_x -1.0) _returnvalue_x) (`KismetMathLibrary.RandomFloatInRange` (* _returnvalue_y -1.0) _returnvalue_y)) (`SceneComponent.K2_GetComponentLocation` (`self.Box`)))) "AdjustIfPossibleButDontSpawnIfColliding" "MultiplyWithRoot" null 10.0 10.0 null))

(fn `UserConstructionScript`)