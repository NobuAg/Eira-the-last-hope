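; BP_Checkpoint is a checkpoint actor that records a respawn point for the player and can open a checkpoint menu.
; On first overlap with BP_Eira, it activates and stores its transform, name and a has-checkpoint flag in BP_GICheckpoint, the game instance.
; Its Checkpoint input opens UW_MenuCheckpoint in UI-only mode and disables actor input, but only if PlayerDetected is true; nothing in these graphs sets that flag.
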(event `self.ReceiveBeginPlay`
  (`self.EnableInput` (`GameplayStatics.GetPlayerController` 0)))

(event `self.DetectPlayer.OnComponentBeginOverlap`
  (params (OverlappedComponent :type "PrimitiveComponent Object Reference") (OtherActor :type "Actor Object Reference") (OtherComp :type "PrimitiveComponent Object Reference") (OtherBodyIndex :type Integer) (bFromSweep :type Boolean) (SweepResult :type "HitResult Structure (by ref)"))
  (cast `/Game/Blueprints/BP_Eira` OtherActor)
  (if (not (`self.bIsActive`))
    (set `self.bIsActive` true)
    (bind _asbp_gicheckpoint (cast `/Game/Blueprints/BP_GICheckpoint` (`GameplayStatics.GetGameInstance`)))
    (set `/Game/Blueprints/BP_GICheckpoint.LastCheckpointTransform` (`self.GetTransform`) _asbp_gicheckpoint)
    (set `/Game/Blueprints/BP_GICheckpoint.HasCheckpoint` true _asbp_gicheckpoint)
    (set `/Game/Blueprints/BP_GICheckpoint.LastCheckpointName` "Checkpoint" _asbp_gicheckpoint)))

(event `InputAction|Checkpoint`
  (params (Key :type "Key Structure"))
  (:`Pressed`
    (if (`self.PlayerDetected`)
      (bind _returnvalue (`|CreateWidget` "/Game/Blueprints/UW_MenuCheckpoint.UW_MenuCheckpoint_C"))
      (`UserWidget.AddToViewport` _returnvalue 0)
      (`self.DisableInput` (`GameplayStatics.GetPlayerController` 0))
      (`WidgetBlueprintLibrary.SetInputMode_UIOnlyEx` null null))))

(fn `UserConstructionScript`)