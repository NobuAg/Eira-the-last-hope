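; Boss encounter trigger that plays a dialogue with the player character Eira before starting the Vaelith fight.
; When Eira enters the Box_Charla volume, it stops her movement and input, then opens a focused WBP_Dialogo widget once, guarded by Iniciado.
; The dialogue's finish event re-enables her input, though it reapplies UI-only input mode, and switches Vaelith's boss state.
; The boss reference is captured only when Vaelith overlaps this actor.
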(event `self.ReceiveActorBeginOverlap`
  (params (OtherActor :type "Actor Object Reference"))
  (bind _asbp_vaelith (cast `/Game/Textures/Characters/Vaelith/Animations/BP_Vaelith` OtherActor))
  (set `self.Boss Ref` _asbp_vaelith))

(event `self.Box_Charla.OnComponentBeginOverlap`
  (params (OverlappedComponent :type "PrimitiveComponent Object Reference") (OtherActor :type "Actor Object Reference") (OtherComp :type "PrimitiveComponent Object Reference") (OtherBodyIndex :type Integer) (bFromSweep :type Boolean) (SweepResult :type "HitResult Structure (by ref)"))
  (bind _asbp_eira (cast `/Game/Blueprints/BP_Eira` OtherActor))
  (set `/Game/Blueprints/BP_Eira.Semueve?` false _asbp_eira)
  (`self.DisableInput` _asbp_eira null)
  (if (not (`self.Iniciado??`))
    (set `self.Iniciado??` true)
    (bind _returnvalue (`|CreateWidget` "/Game/Blueprints/WBP_Dialogo.WBP_Dialogo_C"))
    (`UserWidget.AddToViewport` _returnvalue 0)
    (`WidgetBlueprintLibrary.SetInputMode_UIOnlyEx` (`GameplayStatics.GetPlayerController` 0) (`self.WidgetDialogo`))
    (bind _output_get (set `self.WidgetDialogo` _returnvalue))
    (`Widget.SetKeyboardFocus` (`self.WidgetDialogo`))
    (add `/Game/Blueprints/WBP_Dialogo.OnDialogoFinish` _output_get (delegate `On_DialogoFinish`))))

(event `On_DialogoFinish`
  (`WidgetBlueprintLibrary.SetInputMode_UIOnlyEx` (`GameplayStatics.GetPlayerController` 0) (`self.WidgetDialogo`))
  (`self.EnableInput` (stale `self.Box_Charla.OnComponentBeginOverlap` _asbp_eira) null)
  (`self.IniciarBatalla`))

(event `IniciarBatalla`
  (set `/Game/Textures/Characters/Vaelith/Animations/BP_Vaelith.VaelithStatesBoss` "NewEnumerator1" (`self.Boss Ref`)))

(fn `UserConstructionScript`)